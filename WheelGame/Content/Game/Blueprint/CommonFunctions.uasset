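; CommonFunctions is a shared helper Blueprint holding a single math function, MapFunction.
; MapFunction linearly remaps an input value from a source range to a target range, scaling its offset by the ratio of the two range widths.
; The result is not clamped to the target range, and a zero-width source range is not guarded against division by zero.
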(fn `Map Function`
  (params (`From Min` :type "Float (double-precision)") (`From Max` :type "Float (double-precision)") (`To Min` :type "Float (double-precision)") (`To Max` :type "Float (double-precision)") (`Input Value` :type "Float (double-precision)"))
  (returns (`Output Value` :type "Float (double-precision)"))
  (locals (`Old Range` :type "Float (double-precision)") (`New Range` :type "Float (double-precision)"))
  (set `local.Old Range` (- `From Max` `From Min`))
  (set `local.New Range` (- `To Max` `To Min`))
  (return (+ (/ (* (- (`local.Input Value`) (`local.From Min`)) (`local.New Range`)) (`local.Old Range`)) (`local.To Min`))))