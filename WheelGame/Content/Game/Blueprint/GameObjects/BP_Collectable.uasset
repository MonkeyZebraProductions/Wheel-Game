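; BP_Collectable is a pickup that bobs in place and is consumed on overlap.
; On BeginPlay, the RotateCollectable timeline drives the Cube's relative Z location from its Height track; despite the name, the rotation step is disconnected and never runs.
; On actor overlap, it sends a CollectObject message to the other actor and destroys itself, without filtering who overlapped.
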(event `self.ReceiveBeginPlay`
  (bind (_direction _rotation _height) (`Timeline|Rotate Collectable`)
    (:`Update`
      (`SceneComponent.K2_SetRelativeLocation` (`self.Cube`) (`KismetMathLibrary.MakeVector` 0.0 0.0 (+ (* _height 20.0) -30.0)) false false))))

(event `self.ReceiveActorBeginOverlap`
  (params (OtherActor :type "Actor Object Reference"))
  (message `/Game/Game/Blueprint/BlueprintInterfaces/BI_Player.Call Collect Object` OtherActor)
  (`self.K2_DestroyActor`))

(fn `UserConstructionScript`)