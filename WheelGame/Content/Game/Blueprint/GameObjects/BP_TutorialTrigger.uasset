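; Tutorial trigger volume that all but freezes the overlapping actor to show a tutorial prompt until it is marked as read.
; On overlap, it slows that actor through CustomTimeDilation, passes keyboard text to its widget component and unhides it after a short delay.
; Charge, Left or Jump input restores the stored actor's speed and sets TutorialRead to block later triggers, but does not hide the widget.
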(event `self.ReceiveActorBeginOverlap`
  (params (OtherActor :type "Actor Object Reference"))
  (bind _widget (`self.Widget`))
  (if (not (`self.TutorialRead`))
    (bind _output_get (set `self.Player` OtherActor))
    (set `Actor.CustomTimeDilation` 0.0025 _output_get)
    (message `/Game/Game/Blueprint/BlueprintInterfaces/BI_UI.Set Tutorial Info` (`WidgetComponent.GetUserWidgetObject` _widget) (`self.Keyboard Text`) null false)
    (`KismetSystemLibrary.Delay` 0.5)
    (`SceneComponent.SetHiddenInGame` _widget false false)))

(event `EnhancedInput|/Game/Game/Blueprint/Input/Actions/IA_Charge`
  (params (ActionValue :type Boolean) (ElapsedSeconds :type "Float (double-precision)") (TriggeredSeconds :type "Float (double-precision)") (InputAction :type "InputAction Object Reference" :default "/Game/Game/Blueprint/Input/Actions/IA_Charge.IA_Charge"))
  (bind _player (`self.Player`))
  (:`Started`
    (`/Engine/EditorBlueprintResources/StandardMacros.IsValid` _player :!label _label
      (:`Is Valid`
        (set `Actor.CustomTimeDilation` 1.0 _player)
        (set `self.TutorialRead` true)))))

(event `EnhancedInput|/Game/Game/Blueprint/Input/Actions/IA_Left`
  (params (ActionValue :type Boolean) (ElapsedSeconds :type "Float (double-precision)") (TriggeredSeconds :type "Float (double-precision)") (InputAction :type "InputAction Object Reference" :default "/Game/Game/Blueprint/Input/Actions/IA_Left.IA_Left"))
  (:`Started`
    (goto _label)))

(event `EnhancedInput|/Game/Game/Blueprint/Input/Actions/IA_Jump`
  (params (ActionValue :type Boolean) (ElapsedSeconds :type "Float (double-precision)") (TriggeredSeconds :type "Float (double-precision)") (InputAction :type "InputAction Object Reference" :default "/Game/Game/Blueprint/Input/Actions/IA_Jump.IA_Jump"))
  (:`Started`
    (goto _label)))

(fn `UserConstructionScript`)