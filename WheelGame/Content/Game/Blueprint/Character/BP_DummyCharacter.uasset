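; BP_DummyCharacter is a stand-in character that drives the main canvas HUD with simple test inputs and events.
; BeginPlay creates WBP_MainCanvas, D toggles constant +Y movement on Tick, and R sends a fixed charge level to the HUD.
; CallCheckpointHit shows a checkpoint message with placeholder values.
; CallCollectObject updates the HUD's collectable count and only prints a charge-increase message at each set increment.
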(event `self.ReceiveBeginPlay`
  (bind _returnvalue (`|CreateWidget` "/Game/Game/Blueprint/UIWidgets/WBP_MainCanvas.WBP_MainCanvas_C" (`self.GetLocalViewingPlayerController`)))
  (bind _output_get (set `self.MainCanvas` _returnvalue))
  (`UserWidget.AddToPlayerScreen` _output_get 0))

(event `self.ReceiveTick`
  (params (DeltaSeconds :type "Float (single-precision)"))
  (if (`self.Is Moving`)
    (`self.AddMovementInput` (0.0 1.0 0.0))))

(event `Key|D`
  (params (Key :type "Key Structure"))
  (:`Pressed`
    (bind _isa (`/Engine/EditorBlueprintResources/StandardMacros.FlipFlop`)
      (:`A`
        _)
      (:`B`
        _))
    (set `self.Is Moving` _isa)))

(event `/Game/Game/Blueprint/BlueprintInterfaces/BI_Player.Call Checkpoint Hit`
  (message `/Game/Game/Blueprint/BlueprintInterfaces/BI_UI.Show Checkpoint Time` (`self.MainCanvas`) 0 0.0))

(event `Key|R`
  (params (Key :type "Key Structure"))
  (:`Pressed`
    (message `/Game/Game/Blueprint/BlueprintInterfaces/BI_UI.Set Charge Level` (`self.MainCanvas`) 3)))

(event `/Game/Game/Blueprint/BlueprintInterfaces/BI_Player.Call Collect Object`
  (bind _result (`/Engine/EditorBlueprintResources/StandardMacros.IncrementInt` (`self.Collectables`))
    (:`  `
      (bind _output_get (set `self.Collectables` _result))
      (message `/Game/Game/Blueprint/BlueprintInterfaces/BI_UI.Set Collectable Number` (`self.MainCanvas`) _output_get)
      (if (== (mod _output_get (`self.Increase Charge Increment`)) 0)
        (`KismetSystemLibrary.PrintString` "Increase Max Charge Level")))))

(fn `UserConstructionScript`)