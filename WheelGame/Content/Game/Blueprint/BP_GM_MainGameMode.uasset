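; BP_GM_MainGameMode is a game mode that persists per-checkpoint times through a BP_SaveGame object.
; On BeginPlay it asynchronously loads the default slot, creating a new save object in memory if loading fails.
; SaveCurrentCheckpointTime writes a time at the checkpoint index, growing the array as needed, then saves asynchronously.
; LoadCurrentCheckpointTime returns the stored time and whether it exists, falling back to zero for invalid indices.
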(event `self.ReceiveBeginPlay`
  (bind (_savegame _bsuccess) (`AsyncActionHandleSaveGame.AsyncLoadGameFromSlot` (`self.Default`))
    (:`Completed`
      (if _bsuccess
        (bind _asbp_save_game (cast `/Game/Game/Blueprint/GameObjects/BP_SaveGame` _savegame))
        (set `self.SaveGameInstance` _asbp_save_game)
        (`KismetSystemLibrary.PrintString` "SAVE GAME PRESENT" true true (struct :`R` 0.051391 :`G` 1.0 :`A` 1.0))
        (else
          (bind _returnvalue (`GameplayStatics.CreateSaveGameObject` "/Game/Game/Blueprint/GameObjects/BP_SaveGame.BP_SaveGame_C"))
          (set `self.SaveGameInstance` _returnvalue)
          (`KismetSystemLibrary.PrintString` "NO SAVE GAME PRESENT" true true (struct :`R` 1.0 :`B` 0.107587 :`A` 1.0)))))))

(event `/Game/Game/Blueprint/BlueprintInterfaces/BI_GameMode.Save Current Checkpoint Time`
  (params (`Checkpoint Index` :type Integer) (`Checkpoint Time` :type "Float (double-precision)"))
  (`KismetArrayLibrary.Array_Set` (`/Game/Game/Blueprint/GameObjects/BP_SaveGame.CheckpointTimes` (`self.SaveGameInstance`)) `Checkpoint Index` `Checkpoint Time` true)
  (`AsyncActionHandleSaveGame.AsyncSaveGameToSlot` (`self.SaveGameInstance`) (`self.Default`)
    (:`Completed`
      (`KismetSystemLibrary.PrintString` "HII"))))

(fn `Load Current Checkpoint Time`
  (params (CheckpointIndex :type Integer))
  (returns (CheckpointTime :type "Float (double-precision)") (`Time Exists?` :type Boolean))
  (bind _checkpointtimes (`/Game/Game/Blueprint/GameObjects/BP_SaveGame.CheckpointTimes` (`self.SaveGameInstance`)))
  (bind _returnvalue (`KismetArrayLibrary.Array_IsValidIndex` _checkpointtimes CheckpointIndex))
  (return (`KismetMathLibrary.SelectFloat` (`|GetArrayItem` _checkpointtimes CheckpointIndex) 0.0 _returnvalue) _returnvalue))

(fn `UserConstructionScript`)