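; BP_CubeGenerator is a tool actor that builds a wall-like grid of instanced static meshes in the local Y-Z plane.
; The construction script clears and rebuilds the instances from CountY, CountZ and Size, giving each a random quarter-turn yaw.
; It resizes and offsets a Box component to follow the grid, using BoxExtents.
; Refresh is reset afterwards, but its gating branch is disconnected, so every construction re-randomizes the layout.
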(fn `UserConstructionScript`
  (locals (Y :type Integer) (Z :type Integer :default 0) (Rotation :type "Rotator Structure" :default (struct)))
  (bind (_size_x _size_y) (`KismetMathLibrary.BreakVector2D` (`self.Size`)))
  (bind (_returnvalue_x _returnvalue_y) (`KismetMathLibrary.BreakVector2D` (/ (`self.Size`) 2.0)))
  (`InstancedStaticMeshComponent.ClearInstances` (`self.InstancedStaticMesh`))
  (for _index (range 1 (+ (`self.CountY`) 1))
    (set `local.Y` _index)
    (for _index_2 (range 1 (+ (`self.CountZ`) 1))
      (set `local.Z` _index_2)
      (`|ExecutionSequence`
        (:`then_0`
          (set `local.Rotation` (`KismetMathLibrary.MakeRotator` 0.0 0.0 (* (`KismetMathLibrary.RandomInteger` 4) 90.0))))
        (:`then_1`
          (`InstancedStaticMeshComponent.AddInstance` (`self.InstancedStaticMesh`) (`KismetMathLibrary.MakeTransform` (- (`KismetMathLibrary.MakeVector` 0.0 (* (`local.Y`) _size_x) (* _size_y (`local.Z`))) (`KismetMathLibrary.MakeVector` 0.0 _returnvalue_x _returnvalue_y)) (`local.Rotation`)) false)
          (`BoxComponent.SetBoxExtent` (`self.Box`) (* (`KismetMathLibrary.MakeVector` 1.0 (`KismetMathLibrary.Conv_IntToDouble` (`local.Y`)) (`KismetMathLibrary.Conv_IntToDouble` (`local.Z`))) (`KismetMathLibrary.Conv_DoubleToVector` (`self.Box Extents`))) true)
          (`SceneComponent.K2_SetRelativeLocation` (`self.Box`) (* (`KismetMathLibrary.MakeVector` 0.0 (`KismetMathLibrary.Conv_IntToDouble` (`local.Y`)) (`KismetMathLibrary.Conv_IntToDouble` (`local.Z`))) (`KismetMathLibrary.Conv_DoubleToVector` (`self.Box Extents`))) false false)
          (`SceneComponent.K2_SetRelativeLocation` (`self.Box`) (* (`KismetMathLibrary.MakeVector` 0.0 (`KismetMathLibrary.Conv_IntToDouble` (`local.Y`)) (`KismetMathLibrary.Conv_IntToDouble` (`local.Z`))) (`KismetMathLibrary.Conv_DoubleToVector` (`self.Box Extents`))) false false)))))
  (set `self.Refresh` false))